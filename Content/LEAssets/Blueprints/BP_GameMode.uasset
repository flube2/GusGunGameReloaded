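; Game mode Blueprint that tracks the score and restarts the level when the player wins.
; IncreaseScore adds points to Score, then checks it against a hard-coded threshold of 100.
; On a win it shows the WBP_UI_Win widget, waits briefly, then reopens the current level by name.
; Nothing guards the win check, so further score gains during the delay retrigger it.
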(event Custom|DisplayWinMessage
  ;[1 1 1] Win and Restart
  (bind _returnvalue (UserInterface|CreateWidget "/Game/LEAssets/UI/WBP_UI_Win.WBP_UI_Win_C")) ; Make message UI
  (UserInterface|Viewport|AddtoViewport _returnvalue 1) ; Display message UI
  (Utilities|FlowControl|Delay 3.0) ; Wait a few seconds before restarting so player can read
  (CallFunction|RestartLevel) ; Call custom restart level function
)

(event Custom|CheckScoreForWin
  (params (PointsToWin :type Integer))
  ;[1 1 1] Check for win conditions scorewise
  (if (<= PointsToWin (Variables|Default|GetScore)) ; If score is high enough win, else do nothing
    (CallFunction|DisplayWinMessage) ; If player has won, call custom win UI function
  ))

(event Custom|RestartLevel
  ;[1 1 1] Restart Current Level
  (bind _returnvalue (Game|GetCurrentLevelName true)) ; Get current level's name
  (Game|OpenLevel(byName) (Utilities|String|StringToName _returnvalue)) ; Open the current level / "restart"
)

(event Custom|IncreaseScore
  (params (NumPointsToAdd :type Integer))
  ;[1 1 1] Increase Current Score
  (Variables|Default|SetScore (+ NumPointsToAdd (Variables|Default|GetScore))) ; Update the current score
  (CallFunction|CheckScoreforWin 100) ; Call custom function to check if score is high enough to win
)

(fn ConstructionScript)