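; BP_Wedge is a numbered wedge in the level selector that opens its matching level when hit.
; On Hit, it looks up WedgeNumber in LevelsAvailable and, if found, opens the map named "Level" plus that number.
; Otherwise it only prints an on-screen "Loading Level" message with the number.
; A separate LoadLevelSelector function opens the LevelSelector map but is not called within this Blueprint.
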(event EventBeginPlay)

(event Collision|EventHit
  (params (MyComp :type Primitive%20Component%20Object%20Reference) (Other :type Actor%20Object%20Reference) (OtherComp :type Primitive%20Component%20Object%20Reference) (bSelfMoved :type Boolean) (HitLocation :type Vector :default "0, 0, 0") (HitNormal :type Vector :default "0, 0, 0") (NormalImpulse :type Vector :default "0, 0, 0") (Hit :type Hit%20Result%20Structure%20%28by%20ref%29))
  (bind _wedgenumber (Variables|Default|GetWedgeNumber))
  (if (Utilities|Set|Contains (Variables|Default|GetLevelsAvailable) _wedgenumber)
    (CallFunction|LoadWedgeLevel)
    (else
      (Development|PrintString (Utilities|String|Append (Utilities|String|Append (Utilities|String|MakeLiteralString "Loading Level ") (Utilities|String|ToString(Integer) _wedgenumber)) "....") true false "(R=1.000000,G=0.993680,B=0.000000,A=1.000000)"))))

(fn ConstructionScript)

(fn LoadLevelSelector
  (Game|OpenLevel(byName) "LevelSelector"))

(fn LoadWedgeLevel
  (Game|OpenLevel(byName) (Utilities|String|StringToName (Utilities|String|Append (Utilities|String|MakeLiteralString "Level") (Utilities|String|ToString(Integer) (Variables|Default|GetWedgeNumber))))))