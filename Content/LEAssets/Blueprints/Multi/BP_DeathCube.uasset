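; BP_DeathCube is a harmful black cube that costs the player health when touched or struck.
; Its box collider calls DestroyBlackCube when the player pawn overlaps it or when any hit registers.
; That event plays the Invalid_Action sound, destroys the actor, then decreases health on player 0's G3RPlayerState by BlackCubeEffectValue, whatever caused the hit.
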(event OnComponentBeginOverlap(BoxCollider)
  (params (OverlappedComponent :type Primitive%20Component%20Object%20Reference) (OtherActor :type Actor%20Object%20Reference) (OtherComp :type Primitive%20Component%20Object%20Reference) (OtherBodyIndex :type Integer) (bFromSweep :type Boolean) (SweepResult :type Hit%20Result%20Structure%20%28by%20ref%29))
  ;[1 1 1] On collision with player...
  (if (== OtherActor (Game|GetPlayerCharacter 0)) ; If colliding object is the player...
    (CallFunction|DestroyBlackCube) ; Call custom destroy function
  ))

(event OnComponentHit(BoxCollider)
  (params (HitComponent :type Primitive%20Component%20Object%20Reference) (OtherActor :type Actor%20Object%20Reference) (OtherComp :type Primitive%20Component%20Object%20Reference) (NormalImpulse :type Vector :default "0, 0, 0") (Hit :type Hit%20Result%20Structure%20%28by%20ref%29))
  ;[1 1 1] When hit...
  (CallFunction|DestroyBlackCube) ; Call custom Destroy function
)

(event Custom|DestroyBlackCube
  ;[1 1 1] Destroy
  (Audio|PlaySoundatLocation "/Engine/VREditor/Sounds/UI/Invalid_Action.Invalid_Action" "0, 0, 0" "0, 0, 0" 2.0 1.0 0.0 0 0 0) ; Play a sound effect unique to yellow cubes and blue spheres
  (Actor|DestroyActor) ; Destroy self.
  (bind _asg3rplayer_state (Utilities|Casting|CastToG3RPlayerState (Variables|/Script/Engine.Controller|GetPlayerState (Game|GetPlayerController 0))))
  (Default|DecreaseHealth _asg3rplayer_state (Math|Conversions|ToFloat(Integer) (Variables|Default|GetBlackCubeEffectValue))))

(fn ConstructionScript)