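; Pickup spawn manager actor that periodically scatters random pickups around the level.
; On BeginPlay a looping timer fires SpawnFourRandom every SpawnInterval, which nests down to four SpawnOneRandom calls.
; Each call spawns a random class from PickUpSpawnOptions at a random SpawnLocations actor, skipping the spawn if colliding, and sets a limited LifeSpan on it.
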(event EventBeginPlay
  (Utilities|Time|SetTimerbyFunctionName 0 "SpawnFourRandom" (Variables|Default|GetSpawnInterval) true))

(event Collision|EventActorBeginOverlap
  (params (OtherActor :type Actor%20Object%20Reference)))

(event EventTick
  (params (DeltaSeconds :type Float%20%28single-precision%29)))

(fn ConstructionScript)

(fn SpawnOneRandom
  (bind _spawnlocations (Variables|Default|GetSpawnLocations))
  (bind _pickupspawnoptions (Variables|Default|GetPickUpSpawnOptions))
  (bind _returnvalue (Game|SpawnActorfromClass (Utilities|Array|Get(acopy) _pickupspawnoptions (Math|Random|RandomIntegerinRange 0 (- (Utilities|Array|Length _pickupspawnoptions) 1))) (Math|Transform|MakeTransform (Transformation|GetActorLocation (Utilities|Array|Get(acopy) _spawnlocations (Math|Random|RandomIntegerinRange 0 (- (Utilities|Array|Length _spawnlocations) 1)))) "0, 0, 0" (Variables|Default|GetScale)) "DontSpawnIfColliding" 0 0))
  (Actor|SetLifeSpan _returnvalue (Variables|Default|GetLifeSpan)))

(fn SpawnTwoRandom
  (CallFunction|SpawnOneRandom)
  (CallFunction|SpawnOneRandom))

(fn SpawnFourRandom
  (CallFunction|SpawnTwoRandom)
  (CallFunction|SpawnTwoRandom))