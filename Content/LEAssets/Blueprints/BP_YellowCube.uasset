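; BP_YellowCube is a score pickup cube that is destroyed on contact and adds its point value to the game score.
; Its box collider triggers DestroyYellowCube when the player pawn overlaps it, or on any hit regardless of what struck it.
; That event plays the Invalid_Action sound, destroys the actor, then casts the game mode to BP_GameMode and calls IncreaseScore with YellowCubePointValue.
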(event OnComponentBeginOverlap(BoxCollider)
  (params (OverlappedComponent :type Primitive%20Component%20Object%20Reference) (OtherActor :type Actor%20Object%20Reference) (OtherComp :type Primitive%20Component%20Object%20Reference) (OtherBodyIndex :type Integer) (bFromSweep :type Boolean) (SweepResult :type Hit%20Result%20Structure%20%28by%20ref%29))
  (if (== OtherActor (Game|Player|GetPlayerPawn 0))
    (CallFunction|DestroyYellowCube)))

(event OnComponentHit(BoxCollider)
  (params (HitComponent :type Primitive%20Component%20Object%20Reference) (OtherActor :type Actor%20Object%20Reference) (OtherComp :type Primitive%20Component%20Object%20Reference) (NormalImpulse :type Vector :default "0, 0, 0") (Hit :type Hit%20Result%20Structure%20%28by%20ref%29))
  (CallFunction|DestroyYellowCube))

(event Custom|DestroyYellowCube
  (Audio|PlaySoundatLocation "/Engine/VREditor/Sounds/UI/Invalid_Action.Invalid_Action" "0, 0, 0" "0, 0, 0" 2.0 1.0 0.0 0 0 0)
  (Actor|DestroyActor)
  (bind _asbp_game_mode (Utilities|Casting|CastToBP_GameMode (Game|GetGameMode)))
  (Default|IncreaseScore _asbp_game_mode (Variables|Default|GetYellowCubePointValue)))

(event EventBeginPlay)

(event EventTick
  (params (DeltaSeconds :type Float%20%28single-precision%29)))

(fn ConstructionScript)