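; BP_Shield is a Level02 shield actor that loses health when hit and is linked to a MajorStar reference.
; Hits on its box collider, gated by the TakeDamage flag, subtract a fixed amount of health.
; When the next hit would drop health to zero or below, it destroys itself and sets MajorStar to a fixed scale.
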(event OnComponentHit(BoxCollider)
  (params (HitComponent :type Primitive%20Component%20Object%20Reference) (OtherActor :type Actor%20Object%20Reference) (OtherComp :type Primitive%20Component%20Object%20Reference) (NormalImpulse :type Vector :default "0, 0, 0") (Hit :type Hit%20Result%20Structure%20%28by%20ref%29))
  (if (Variables|Default|GetTakeDamage)
    (CallFunction|DecreaseShieldHealth)))

(fn ConstructionScript)

(fn DecreaseShieldHealth
  (if (<= (- (Variables|Default|GetHealth) 10) 0)
    (CallFunction|DestroyShield)
    (else
      (Variables|Default|SetHealth (- (Variables|Default|GetHealth) 10)))))

(fn DestroyShield
  (Actor|DestroyActor)
  (Transformation|SetActorScale3D (Variables|Default|GetMajorStar) "5.000000,5.000000,5.000000"))