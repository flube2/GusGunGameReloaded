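; BP_ShieldDamageTrigger is a Level02 trigger actor that makes a referenced Shield vulnerable once the player has earned enough points.
; When the player character begins overlapping it, it reads CurrentScore from the G3RPlayerState and compares it to PointsToDisable.
; At or above that threshold it sets the Shield's TakeDamage flag to true and never clears it.
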(event Collision|EventActorBeginOverlap
  (params (OtherActor :type Actor%20Object%20Reference))
  (bind _returnvalue (Game|GetPlayerCharacter 0))
  (if (== OtherActor _returnvalue)
    (bind _asg3rplayer_state (Utilities|Casting|CastToG3RPlayerState (Variables|/Script/Engine.Pawn|GetPlayerState _returnvalue)))
    (if (>= (Variables|/Game/LEAssets/Core/G3RPlayerState.G3RPlayerState_C|GetCurrentScore _asg3rplayer_state) (Variables|Default|GetPointsToDisable))
      (Variables|/Game/LEAssets/Blueprints/Level02/BP_Shield.BP_Shield_C|SetTakeDamage (Variables|Default|GetShield) true))))

(fn ConstructionScript)