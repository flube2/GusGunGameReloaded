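; Game mode that tracks the player's score and ends the level with a win once it reaches a fixed threshold.
; IncreaseScore adds points and immediately checks the total against a hardcoded target of 100.
; Reaching the target shows the WBP_UI_Win widget, waits a few seconds, then reopens the current level by name to restart it.
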(event Custom|DisplayWinMessage
  (bind _returnvalue (UserInterface|CreateWidget "/Game/WBP_UI_Win.WBP_UI_Win_C"))
  (UserInterface|Viewport|AddtoViewport _returnvalue 1)
  (Utilities|FlowControl|Delay 3.0)
  (CallFunction|RestartLevel))

(event Custom|CheckScoreForWin
  (params (PointsToWin :type Integer))
  (if (<= PointsToWin (Variables|Default|GetScore))
    (CallFunction|DisplayWinMessage)))

(event Custom|RestartLevel
  (bind _returnvalue (Game|GetCurrentLevelName true))
  (Game|OpenLevel(byName) (Utilities|String|StringToName _returnvalue)))

(event Custom|IncreaseScore
  (params (NumPointsToAdd :type Integer))
  (Variables|Default|SetScore (+ NumPointsToAdd (Variables|Default|GetScore)))
  (CallFunction|CheckScoreforWin 100))

(event EventBeginPlay)

(event EventTick
  (params (DeltaSeconds :type Float%20%28single-precision%29)))

(fn ConstructionScript)